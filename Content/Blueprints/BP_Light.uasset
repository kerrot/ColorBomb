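; BP_Light is a light actor that switches on when its trigger box is first overlapped and counts toward a passed-lights total.
; A DoOnce on the box overlap sets the Lighting flag and increments PassedLights on the game mode.
; Tick applies the Lighting flag to the point light's visibility every frame.
; The overlap does not filter which actor triggers it.
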(event `self.ReceiveTick`
  (params (DeltaSeconds :type "Float (single-precision)"))
  (`SceneComponent.SetVisibility` (`self.PointLight`) (`self.Lighting`) false))

(event `self.Box.OnComponentBeginOverlap`
  (params (OverlappedComponent :type "PrimitiveComponent Object Reference") (OtherActor :type "Actor Object Reference") (OtherComp :type "PrimitiveComponent Object Reference") (OtherBodyIndex :type Integer) (bFromSweep :type Boolean) (SweepResult :type "HitResult Structure (by ref)"))
  (`/Engine/EditorBlueprintResources/StandardMacros.DoOnce` false
    (:`Completed`
      (set `self.Lighting` true)
      (bind _asbp_my_game_mode (cast `` (`GameplayStatics.GetGameMode`)))
      (set `/Game/Blueprints/BP_Light.PassedLights` (+ (`/Game/Blueprints/BP_Light.PassedLights` _asbp_my_game_mode) 1) _asbp_my_game_mode))))

(fn `UserConstructionScript`)
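; BP_Character is a player character Blueprint that handles basic movement, jumping and a hold-to-speed-up control.
; MoveForward and MoveRight axes add movement input along control-yaw directions, scaled by the Speed variable.
; Holding Tab raises Speed and releasing it lowers it, changing the input scale rather than the movement component's max speed.
; Jump triggers the built-in jump, and the Damaged event only prints a debug message.
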(event `InputAxis|MoveForward`
  (params (AxisValue :type "Float (single-precision)"))
  ;[1 1 1] キャラクターを移動
  (`self.AddMovementInput` (`KismetMathLibrary.GetForwardVector` (`KismetMathLibrary.MakeRotator` 0.0 0.0 (.yaw (`self.GetControlRotation`)))) (* AxisValue (`self.Speed`))))

(event `InputAxis|MoveRight`
  (params (AxisValue :type "Float (single-precision)"))
  ;[1 1 1] キャラクターを移動
  (`self.AddMovementInput` (`KismetMathLibrary.GetRightVector` (`KismetMathLibrary.MakeRotator` 0.0 0.0 (.yaw (`self.GetControlRotation`)))) (* AxisValue (`self.Speed`))))

(event `Key|Tab`
  (params (Key :type "Key Structure" :default "AnyKey"))
  ;[1 1 1] キャラクターを移動
  (:`Pressed`
    (set `self.Speed` 0.7))
  (:`Released`
    (set `self.Speed` 0.5)))

(event `InputAction|Jump`
  (params (Key :type "Key Structure" :default "AnyKey"))
  ;[1 1 1] ジャンプ
  (:`Pressed`
    (`self.Jump`)))

(event `Damaged`
  (`KismetSystemLibrary.PrintString` "Damaged"))

(fn `UserConstructionScript`)
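; PlayerControl is a player Blueprint that handles pausing, shooting and taking damage.
; The Pause input adds MainGameWidget to the viewport and pauses the game, guarded by a shown flag that this graph never resets.
; The P key spawns a Bullet at the spawn arrow's location, without using its rotation.
; The Damage event decrements and prints Hp, then prints Game Over and pauses when it equals zero.
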(event `InputAction|Pause`
  (params (Key :type "Key Structure" :default "AnyKey"))
  (:`Pressed`
    (if (not (`self.IsScreenShown`))
      (bind _returnvalue (`|CreateWidget` "/Game/Blueprints/Main/MainGameWidget.MainGameWidget_C"))
      (`UserWidget.AddToViewport` _returnvalue 0)
      (set `self.IsScreenShown` true)
      (`GameplayStatics.SetGamePaused` true))))

(event `Key|P`
  (params (Key :type "Key Structure" :default "AnyKey"))
  (:`Pressed`
    (`|SpawnActorFromClass` "/Game/Blueprints/ShootPoint/Bullet.Bullet_C" (`KismetMathLibrary.Conv_VectorToTransform` (`SceneComponent.GetSocketLocation` (`self.SpwanArrow`) "None")) "Undefined" "OverrideRootScale")))

(event `Damage`
  (bind _output_get (set `self.Hp` (- (`self.Hp`) 1.0)))
  (`KismetSystemLibrary.PrintString` (`KismetStringLibrary.Conv_DoubleToString` _output_get))
  (if (== _output_get 0.0)
    (`KismetSystemLibrary.PrintString` "Game Over")
    (`GameplayStatics.SetGamePaused` true)))

(fn `UserConstructionScript`)
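; Bullet projectile that damages Enemy actors on overlap and destroys itself when it hits an Enemy or a BoundaryBox.
; The construction script sets ProjectileMovement's local velocity from the first ShootPoint, deriving X from horizontal distance, height and gravity.
; HitEvent subtracts Damage from the Enemy's Health, destroys it at zero or below, and otherwise prints the remaining health.
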(event `self.ReceiveActorBeginOverlap`
  (params (OtherActor :type "Actor Object Reference"))
  (`self.HitEvent` OtherActor OtherActor))

(fn `HitEvent`
  (params (BoundaryActor :type "Actor Object Reference") (TestEnemyActor :type "Actor Object Reference"))
  ;[1 1 1] If hit the boundary
  (cast `/Game/Blueprints/ShootPoint/BoundaryBox` BoundaryActor
    (:`then`
      (`KismetSystemLibrary.PrintString` "hit!!")
      (`self.K2_DestroyActor`))
    (:`CastFailed`
      (bind _asenemy (cast `/Game/Blueprints/Main/Enemy` TestEnemyActor))
      (bind _output_get (set `/Game/Blueprints/Main/Enemy.Health` (- (`/Game/Blueprints/Main/Enemy.Health` _asenemy) (`self.Damage`)) _asenemy))
      (if (<= _output_get 0.0)
        (`self.K2_DestroyActor` _asenemy)
        (`self.K2_DestroyActor`)
        (else
          (`KismetSystemLibrary.PrintString` (`KismetStringLibrary.Conv_DoubleToString` _output_get))
          (`self.K2_DestroyActor`))))))

(fn `UserConstructionScript`
  (locals (NewLocalVar_0 :type "Vector Structure" :default (100.0 0.0 0.0)))
  (bind (_returnvalue_x _returnvalue_y _returnvalue_z) (`KismetMathLibrary.BreakVector` (`self.K2_GetActorLocation`)))
  (bind _outactors (`GameplayStatics.GetAllActorsOfClass` "/Game/Blueprints/ShootPoint/ShootPoint.ShootPoint_C"))
  (bind _asshoot_point (cast `/Game/Blueprints/ShootPoint/ShootPoint` (`KismetArrayLibrary.Array_Get` _outactors)))
  (bind (_returnvalue_x_2 _returnvalue_y_2) (`KismetMathLibrary.BreakVector` (`self.K2_GetActorLocation` _asshoot_point)))
  (`ProjectileMovementComponent.SetVelocityInLocalSpace` (`self.ProjectileMovement`) (`KismetMathLibrary.MakeVector` (* (/ (- _returnvalue_x_2 _returnvalue_x) (`KismetMathLibrary.Abs` (/ (* (+ _returnvalue_z 300.0) 2.0) (`MovementComponent.GetGravityZ` (`self.ProjectileMovement`))))) 2.0) _returnvalue_y_2 -9.8)))
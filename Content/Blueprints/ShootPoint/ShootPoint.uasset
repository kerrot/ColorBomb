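; ShootPoint is an actor meant to be a movable target point, with a debug line trace drawn to it from the player's capsule every tick.
; W/S and A/D set flags that input axis events check to shift it along world X and Y, scaled by delta time and Speed or TurnRate.
; The trace and move functions reference a ShootPoint cast from GetAllActorsOfClass, but those lookup chains are disconnected and never execute.
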(event EventTick
  (params (DeltaSeconds :type Float%20%28single-precision%29))
  (CallFunction|LineTraceAction))

(event Input|AxisEvents|InputAxisaAxis
  (params (AxisValue :type Float%20%28single-precision%29))
  (if (Variables|Default|GetaPressed)
    (Input|EnableInput 0)
    (CallFunction|MoveLeft)))

(event Input|AxisEvents|InputAxisdAxis
  (params (AxisValue :type Float%20%28single-precision%29))
  (if (Variables|Default|GetdPressed)
    (Input|EnableInput 0)
    (CallFunction|MoveRight)))

(event Input|AxisEvents|InputAxiswAxis
  (params (AxisValue :type Float%20%28single-precision%29))
  (if (Variables|Default|GetwPressed)
    (Input|EnableInput 0)
    (CallFunction|MoveForward)))

(event Input|AxisEvents|InputAxissAxis
  (params (AxisValue :type Float%20%28single-precision%29))
  (if (Variables|Default|GetsPressed)
    (Input|EnableInput 0)
    (CallFunction|MoveBack)))

(event Input|KeyboardEvents|A
  (params (Key :type Key%20Structure :default "AnyKey"))
  ;[1 1 1] Input
  (:Pressed
    (Variables|Default|SetaPressed true))
  (:Released
    (Variables|Default|SetaPressed false)))

(event Input|KeyboardEvents|D
  (params (Key :type Key%20Structure :default "AnyKey"))
  ;[1 1 1] Input
  (:Pressed
    (Variables|Default|SetdPressed true))
  (:Released
    (Variables|Default|SetdPressed false)))

(event Input|KeyboardEvents|W
  (params (Key :type Key%20Structure :default "AnyKey"))
  ;[1 1 1] Input
  (:Pressed
    (Variables|Default|SetwPressed true))
  (:Released
    (Variables|Default|SetwPressed false)))

(event Input|KeyboardEvents|S
  (params (Key :type Key%20Structure :default "AnyKey"))
  ;[1 1 1] Input
  (:Pressed
    (Variables|Default|SetsPressed true))
  (:Released
    (Variables|Default|SetsPressed false)))

(fn ConstructionScript)

(fn LineTraceAction
  (Collision|LineTraceByChannel (Transformation|GetWorldLocation (Variables|/Script/Engine.Character|GetCapsuleComponent (Game|GetPlayerCharacter 0))) (Transformation|GetActorLocation (stale _asshoot_point)) "TraceTypeQuery1" false 0 "ForOneFrame"))

(fn MoveForward
  (Transformation|SetActorLocation (Math|Vector|MakeVector (+ (.x (Transformation|GetActorLocation (stale _asshoot_point))) (* (Utilities|Time|GetWorldDeltaSeconds) (Variables|Default|Getspeed))) (.y (Transformation|GetActorLocation (stale _asshoot_point))) (.z (Transformation|GetActorLocation (stale _asshoot_point)))) false false))

(fn MoveBack
  (Transformation|SetActorLocation (Math|Vector|MakeVector (- (.x (Transformation|GetActorLocation (stale _asshoot_point))) (* (Utilities|Time|GetWorldDeltaSeconds) (Variables|Default|Getspeed))) (.y (Transformation|GetActorLocation (stale _asshoot_point))) (.z (Transformation|GetActorLocation (stale _asshoot_point)))) false false))

(fn MoveRight
  (Transformation|SetActorLocation (stale _asshoot_point) (Math|Vector|MakeVector (.x (Transformation|GetActorLocation (stale _asshoot_point))) (+ (.y (Transformation|GetActorLocation (stale _asshoot_point))) (* (Utilities|Time|GetWorldDeltaSeconds) (Variables|Default|GetTurnRate))) (.z (Transformation|GetActorLocation (stale _asshoot_point)))) false false))

(fn MoveLeft
  (Transformation|SetActorLocation (stale _asshoot_point) (Math|Vector|MakeVector (.x (Transformation|GetActorLocation (stale _asshoot_point))) (- (.y (Transformation|GetActorLocation (stale _asshoot_point))) (* (Utilities|Time|GetWorldDeltaSeconds) (Variables|Default|GetTurnRate))) (.z (Transformation|GetActorLocation (stale _asshoot_point)))) false false))
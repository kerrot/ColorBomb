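; Enemy spawner that populates a box volume with AI enemies over time, up to a population limit.
; After a start delay on BeginPlay, a looping timer calls Spawn at an interval derived from the spawn rate.
; Spawn counts existing Enemy actors and, if below the cap, spawns a batch of the configured pawn class at random points inside the volume.
; The cap is checked once per batch, so the total can overshoot it.
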(event `self.ReceiveBeginPlay`
  ;[1 1 1] EnemySpawnController
  (`KismetSystemLibrary.Delay` (`self.StartSpawnEnemies`))
  (`KismetSystemLibrary.K2_SetTimer` null "Spawn" (/ 1.0 (`self.EnemiesPerSecond`)) true))

(fn `Spawn`
  (bind _spawnvolume (`self.SpawnVolume`))
  (bind _outactors (`GameplayStatics.GetAllActorsOfClass` "/Game/Blueprints/Enemy/Enemy.Enemy_C"))
  (if (< (`KismetArrayLibrary.Array_Length` _outactors) (`self.MaxEnemies`))
    (for _ (range 1 (+ (`self.EnemyPerSecond`) 1))
      (`AIBlueprintHelperLibrary.SpawnAIFromClass` (`self.EnemyType`) null (`KismetMathLibrary.RandomPointInBoundingBox` (`SceneComponent.K2_GetComponentLocation` _spawnvolume) (`BoxComponent.GetScaledBoxExtent` _spawnvolume)) (struct :`Yaw` 180.0)))))

(fn `UserConstructionScript`)
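; Enemy character blueprint that heads for a target point, takes damage and rewards the player with bombs on death.
; GetEnemyTarget stores the first TargetPoint as Goal, Attack sets CanAttack when within ReachDistance, and EnemyMoveToLocation uses SimpleMoveToLocation until then.
; Attacked subtracts and prints Health, then at zero flags death and adds red, blue and green bomb bounties to PlayerControl.
; Its event graph is empty, leaving these functions uncalled here.
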(event `self.ReceiveBeginPlay`)

(event `self.ReceiveTick`
  (params (DeltaSeconds :type "Float (single-precision)")))

(fn `Attack`
  (set `self.CanAttack` (<= (`self.GetDistanceTo` self (`self.Goal`)) (`self.ReachDistance`))))

(fn `Attacked`
  (params (DamageValue :type "Float (double-precision)" :default 1.0))
  (set `self.BeAttacked` true)
  (bind _output_get (set `self.Health` (- (`self.Health`) DamageValue)))
  (`KismetSystemLibrary.PrintString` (`KismetStringLibrary.Conv_DoubleToString` _output_get))
  (if (<= (`self.Health`) 0.0)
    (set `self.IsDead` true)
    (bind _asplayer_control (cast `/Game/Blueprints/Main/PlayerControl` (`GameplayStatics.GetPlayerCharacter` 0)))
    (bind _asplayer_control_2 (cast `/Game/Blueprints/Main/PlayerControl` (`GameplayStatics.GetPlayerCharacter` 0)))
    (`|ExecutionSequence`
      (:`then_0`
        (set `/Game/Blueprints/Main/PlayerControl.RedBombNumber` (+ (`/Game/Blueprints/Main/PlayerControl.RedBombNumber` _asplayer_control) (`self.RedBombBounds`)) _asplayer_control_2))
      (:`then_1`
        (set `/Game/Blueprints/Main/PlayerControl.BlueBombNumber` (+ (`/Game/Blueprints/Main/PlayerControl.BlueBombNumber` _asplayer_control) (`self.BlueBombBounds`)) _asplayer_control_2))
      (:`then_2`
        (set `/Game/Blueprints/Main/PlayerControl.GreenBombNumber` (+ (`/Game/Blueprints/Main/PlayerControl.GreenBombNumber` _asplayer_control) (`self.GreebBombBounds`)) _asplayer_control_2)))))

(fn `EnemyMoveToLocation`
  (if (not (`self.CanAttack`))
    (if (not (`self.IsDead`))
      (if (`self.CanMove`)
        (`NavigationSystem.SimpleMoveToLocation` (`self.GetController` self) (`self.K2_GetActorLocation` (`self.Goal`)))
        (else
          (`MovementComponent.StopMovementImmediately` (`self.CharacterMovement`)))))))

(fn `GetEnemyTarget`
  (bind _outactors (`GameplayStatics.GetAllActorsOfClass` "/Script/Engine.TargetPoint"))
  (set `self.Goal` (`KismetArrayLibrary.Array_Get` _outactors)))

(fn `UserConstructionScript`)
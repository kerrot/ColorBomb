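; Boss enemy Blueprint that chases and attacks a target, using functions defined outside this graph.
; BeginPlay acquires the target, then each Tick runs a Sequence for movement, attack, hit recovery and death.
; Delays clear the BeAttacked flag and destroy the actor once it is dead and not falling.
; Parent BeginPlay and Tick calls are disabled, so this graph replaces that event logic.
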(event `self.ReceiveBeginPlay`
  (`self.GetEnemyTarget`))

(event `self.ReceiveTick`
  (params (DeltaSeconds :type "Float (single-precision)"))
  (`|ExecutionSequence`
    (:`then_0`
      (`self.EnemyMoveToLocation`))
    (:`then_1`
      (`self.Attack`))
    (:`then_2`
      (if (== (`self.BeAttacked`) true)
        (`KismetSystemLibrary.Delay` 1.0)
        (set `self.BeAttacked` false)))
    (:`then_3`
      (if (`self.IsDead`)
        (if (not (`NavMovementComponent.IsFalling` (`self.GetMovementComponent`)))
          (`KismetSystemLibrary.Delay` 1.2)
          (`self.K2_DestroyActor`))))))

(fn `UserConstructionScript`
  (`parent.UserConstructionScript`))